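; Blueprint from a bone transform example that drives a head-aiming Pitch value toward a target actor.
; Each Tick it takes the direction from the mesh's head socket to TargetActor and compares it with the actor's up vector.
; The arccosine of that dot product, minus 90 degrees, becomes the signed Pitch angle, presumably for bone rotation elsewhere.
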(event `self.ReceiveTick`
  (params (DeltaSeconds :type "Float (single-precision)"))
  (set `self.Pitch` (- (`KismetMathLibrary.DegAcos` (`KismetMathLibrary.Dot_VectorVector` (`KismetMathLibrary.GetDirectionUnitVector` (`SceneComponent.GetSocketLocation` (`self.Mesh`) "head") (`self.K2_GetActorLocation` (`self.TargetActor`))) (`self.GetActorUpVector`))) 90.0)))

(fn `UserConstructionScript`)